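; EyeInteract is an actor Blueprint that shifts its Cube in response to remote messages received over Socket.IO.
; On BeginPlay it binds the "new wind" event to the SocketIO client's generic event handler.
; That handler compares the quoted JSON string against left, right and center, moving the Cube along its relative X axis to either side or back to zero.
; Connection and disconnection, with its reason, are printed for debugging.
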(event OnGenericEvent(SocketIOClient)
  (params (EventName :type String) (MessageJson :type SIO%20Json%20Value%20Object%20Reference))
  (bind _returnvalue (Class|SIOJsonValue|AsString MessageJson))
  (bind _cube (Variables|Default|GetCube))
  (if (Utilities|Enum|Equal(Enum) EventName "new wind")
    (if (Utilities|Enum|Equal(Enum) _returnvalue "\"left\"")
      (Components|MoveComponentTo _cube "10.000000, 0, 0" "0, 0, 0" false false 0.2 false)
      (elif (Utilities|Enum|Equal(Enum) _returnvalue "\"right\"")
        (Components|MoveComponentTo _cube "-10.000000, 0, 0" "0, 0, 0" false false 0.2 false)
        (elif (Utilities|Enum|Equal(Enum) _returnvalue "\"center\"")
          (Components|MoveComponentTo _cube "0.000000, 0, 0" "0, 0, 0" false false 0.2 false))))))

(event OnConnected(SocketIOClient)
  (params (SessionId :type String) (bIsReconnection :type Boolean))
  (Development|PrintString "Connected"))

(event OnDisconnected(SocketIOClient)
  (params (Reason :type ESIOConnectionCloseReason%20Enum :default "CLOSE_REASON_NORMAL"))
  (Development|PrintString (Utilities|String|Append "Disconnected" (Utilities|String|EnumtoString Reason))))

(event EventBeginPlay
  (Class|SocketIOClientComponent|BindEventtoGenericEvent (Variables|Default|GetSocketIOClient) "new wind" "/"))

(event Collision|EventActorBeginOverlap
  (params (OtherActor :type Actor%20Object%20Reference)))

(event EventTick
  (params (DeltaSeconds :type Float%20%28single-precision%29)))

(fn ConstructionScript)